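; Per-floor elevator door frame with sliding outside doors, animated call buttons, floor and arrow displays, a floor plate and optional shaft walls.
; FindElevator box-overlaps vertically for an "Elevator"-tagged actor and passes the call and itself to BP_Elevator.
; A timeline slides the doors using one of five speed tracks, with movement sounds triggered by comparing door position over a short delay.
; Button lights and displays swap materials to show call state, floor and travel direction.
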(event Custom|Call%20Button%20Down%20Light
  (bind _callbuttondown (Variables|Default|GetCallButtonDown))
  ;[1 1 1] Call button light
  ;;[0.1744 1 0] Change the material to turn the button light on or off.
  (if (Variables|Default|GetCallButtonDownLightOn)
    (Rendering|Material|SetMaterial _callbuttondown 0 "/Game/ElevatorSystem/Material/Instances/ButtonLight/MI_ButtonLight_03.MI_ButtonLight_03")
    (Rendering|Material|SetMaterial (Variables|Default|GetCallButtonUp) 0 "/Game/ElevatorSystem/Material/Instances/ButtonLight/MI_ButtonLight_02.MI_ButtonLight_02")
    (else
      (Rendering|Material|SetMaterial _callbuttondown 0 "/Game/ElevatorSystem/Material/Instances/ButtonLight/MI_ButtonLight_02.MI_ButtonLight_02"))))

(event Custom|FindElevator
  (params (IsUpButton :type Boolean))
  (bind _elevatorframe (Variables|Default|GetElevatorFrame))
  (bind _returnvalue (Transformation|GetWorldLocation _elevatorframe))
  ;[1 1 1] Find elevator
  ;;[0.1744 1 0] Find the nearest elevator by tag and send variable values to "BP_Elevator".
  (bind (_outactors _returnvalue_2) (Collision|BoxOverlapActors (Transformation|GetWorldLocation (Variables|Default|GetCollision)) "1.000000,1.000000,100000.000000" (Utilities|Array|MakeArray "ObjectTypeQuery2") 0 :!class /Script/Engine.KismetSystemLibrary))
  (if _returnvalue_2
    (for _array_element _outactors
      (if (Actor|ActorHasTag (.ReturnValue (Actor|FindNearestActor _returnvalue (Utilities|Array|MakeArray _array_element))) "Elevator")
        (bind _asbp_elevator (Utilities|Casting|CastToBP_Elevator (.ReturnValue (Actor|FindNearestActor _returnvalue (Utilities|Array|MakeArray _array_element)))))
        (Default|ElevatorCall _asbp_elevator _returnvalue self IsUpButton)))))

(event Custom|SetFloorPlate
  (params (FloorsBelowGround :type Integer))
  (bind _jambplate (Variables|Default|GetJambPlate))
  ;[1 1 1] Floor plate
  ;;[0.1744 1 0] Show the right plate for each "DoorFrames" index.
  (for (_array_element _array_index) (Variables|Default|GetDoorFrames)
    (if (== _array_element self)
      (Math|Integer|CompareInt FloorsBelowGround
        (:>
          (Components|StaticMesh|SetStaticMesh (Variables|Default|GetFloorPlateNumber) (.Value (Utilities|Map|Find _jambplate (+ _array_index FloorsBelowGround))) :!label _label))
        (:==
          (goto _label))
        (:<
          (Components|StaticMesh|SetStaticMesh (Variables|Default|GetFloorPlateNumber) (.Value (Utilities|Map|Find _jambplate (+ _array_index FloorsBelowGround)))))))))

(event Custom|DoorSound
  (bind _outsidedoorright (Variables|Default|GetOutsideDoorRight))
  (bind _elevatordoormoving (Variables|Default|GetElevatorDoorMoving))
  (bind _returnvalue (Audio|Components|Audio|IsPlaying _elevatordoormoving))
  (bind _relativelocation (Variables|/Script/Engine.SceneComponent|GetRelativeLocation _outsidedoorright))
  (bind _x (Math|Vector|BreakVector _relativelocation))
  ;[1 1 1] Door sound
  ;;[0.1744 1 0] Store X door axis in "DoorMoving"and compare with current door axis to see if its moving.
  (bind _output_get (Variables|Default|SetDoorMoving _x))
  (Utilities|FlowControl|Delay 0.01)
  (if (Math|Float|NearlyEqual(Float) _x _output_get 0.004)
    (if _returnvalue
      (Audio|Components|Audio|Stop (Variables|Default|GetElevatorDoorMoving))
      (Math|Float|CompareFloat _x 3e+01
        (:>
          (Audio|Components|Audio|Play (Variables|Default|GetStopDoorMove_01) 0.0))
        (:==
          (Audio|Components|Audio|Play (Variables|Default|GetStopDoorMove_02) 0.0 :!label _label))
        (:<
          (goto _label))))
    (elif (not _returnvalue)
      (Audio|Components|Audio|Play (Variables|Default|GetElevatorDoorMoving) 0.0))))

(event Custom|FloorDisplayDoorFrame
  (bind _floordisplaymaterialmap (Variables|Default|GetFloorDisplayMaterialMap))
  ;[1 1 1] Floor Display door frame
  ;;[0.1744 1 0] Compare "FloorDisplayNumber" with "FloorDisplayTextureMap" to get what floor number texture to put on the display material.
  (bind _keys (Utilities|Map|Keys _floordisplaymaterialmap))
  (for _array_element _keys
    (Math|Integer|CompareInt _array_element (Variables|Default|GetFloorDisplayNumberDoorFrame)
      (:==
        (if (.ReturnValue (Utilities|Map|Find _floordisplaymaterialmap _array_element))
          (Rendering|Material|SetMaterial (Variables|Default|GetDisplayFloor) 0 (.Value (Utilities|Map|Find _floordisplaymaterialmap _array_element))))))))

(event Custom|CloseOutsideDoor
  (bind _finaloutsidedoorspeed (Variables|Default|GetFinalOutsideDoorSpeed))
  ;[1 1 1] Open/Close outside door
  (bind (_direction _speed_01 _speed_02 _speed_03 _speed_04 _speed_05) (Timeline|DoorSpeedTimeline Reverse)
    (:Update
      (CallFunction|OutSideDoorSpeed _speed_01 _speed_02 _speed_03 _speed_04 _speed_05)
      (Utilities|FlowControl|Sequence
        (:then_0
          (CallFunction|DoorSound)
          (Transformation|SetRelativeLocation (Variables|Default|GetOutsideDoorLeft) (Math|Vector|MakeVector (Math|Float|Lerp 0.0 -56.0 _finaloutsidedoorspeed) 0.0 0.0) false false))
        (:then_1
          (CallFunction|DoorSound)
          (Transformation|SetRelativeLocation (Variables|Default|GetOutsideDoorRight) (Math|Vector|MakeVector (Math|Float|Lerp 0.0 56.0 _finaloutsidedoorspeed) 0.0 0.0) false false))))
    (:Finished
      (CallFunction|DoorSound))))

(event Custom|OpenOutsideDoor
  (bind _finaloutsidedoorspeed (Variables|Default|GetFinalOutsideDoorSpeed))
  ;[1 1 1] Open/Close outside door
  (bind (_direction _speed_01 _speed_02 _speed_03 _speed_04 _speed_05) (Timeline|DoorSpeedTimeline Play)
    (:Update
      (CallFunction|OutSideDoorSpeed _speed_01 _speed_02 _speed_03 _speed_04 _speed_05)
      (Utilities|FlowControl|Sequence
        (:then_0
          (CallFunction|DoorSound)
          (Transformation|SetRelativeLocation (Variables|Default|GetOutsideDoorLeft) (Math|Vector|MakeVector (Math|Float|Lerp 0.0 -56.0 _finaloutsidedoorspeed) 0.0 0.0) false false))
        (:then_1
          (CallFunction|DoorSound)
          (Transformation|SetRelativeLocation (Variables|Default|GetOutsideDoorRight) (Math|Vector|MakeVector (Math|Float|Lerp 0.0 56.0 _finaloutsidedoorspeed) 0.0 0.0) false false))))
    (:Finished
      (CallFunction|DoorSound))))

(event Custom|PushCallButtonUp
  (bind _callbuttonup (Variables|Default|GetCallButtonUp))
  (bind _relativelocation (Variables|/Script/Engine.SceneComponent|GetRelativeLocation _callbuttonup))
  (bind (_x _y _z) (Math|Vector|BreakVector _relativelocation))
  ;[1 1 1] Push call button up
  ;;[0.1744 1 0] Store the initial button location on "ButtonPosition", move the button and move back to the initial location.
  (Audio|Components|Audio|Play (Variables|Default|GetButtonNoise) 0.0)
  (if (Variables|Default|GetCanPushCallButton)
    (Audio|Components|Audio|Play (Variables|Default|GetButtonBip) 0.0)
    (Variables|Default|SetCanPushCallButton false)
    (bind _output_get (Variables|Default|SetButtonPosition _relativelocation))
    (bind _alpha (Timeline|Timeline_3 PlayFromStart)
      (:Update
        (Transformation|SetRelativeLocation _callbuttonup (Math|Vector|MakeVector _x (Math|Float|Lerp _y (- _y 0.07) _alpha) _z) false false))
      (:Finished
        (bind _alpha_2 (Timeline|Timeline_4 PlayFromStart)
          (:Update
            (Transformation|SetRelativeLocation _callbuttonup (Math|Vector|MakeVector (.X (Math|Vector|BreakVector _output_get)) (Math|Float|Lerp (Math|Float|Lerp _y (- _y 0.07) _alpha) (.Y (Math|Vector|BreakVector _output_get)) _alpha_2) (.Z (Math|Vector|BreakVector _output_get))) false false))
          (:Finished
            (Variables|Default|SetCanPushCallButton true)))))))

(event Custom|OutsideDoorSpeed
  (params (Speed%20_01 :type Float%20%28double-precision%29) (Speed_02 :type Float%20%28double-precision%29) (Speed_03 :type Float%20%28double-precision%29) (Speed_04 :type Float%20%28double-precision%29) (Speed_05 :type Float%20%28double-precision%29))
  (bind _setoutsidedoorspeed (Variables|Default|GetSetOutsideDoorSpeed))
  ;[1 1 1] Outside door speed
  ;;[0.1744 1 0] Assign the "SetOutsideDoorSpeed" value to "DoorSpeedTimeline" speed variable, which is inside "OutsideDoorSpeed" event, and assign to "FinalOutsideDoorSpeed".
  (Utilities|FlowControl|Sequence
    (:then_0
      (Math|Integer|CompareInt _setoutsidedoorspeed 1
        (:==
          (Variables|Default|SetFinalOutsideDoorSpeed Speed%20_01))))
    (:then_1
      (Math|Integer|CompareInt _setoutsidedoorspeed 2
        (:==
          (Variables|Default|SetFinalOutsideDoorSpeed Speed_02))))
    (:then_2
      (Math|Integer|CompareInt _setoutsidedoorspeed 3
        (:==
          (Variables|Default|SetFinalOutsideDoorSpeed Speed_03))))
    (:then_3
      (Math|Integer|CompareInt _setoutsidedoorspeed 4
        (:==
          (Variables|Default|SetFinalOutsideDoorSpeed Speed_04))))
    (:then_4
      (Math|Integer|CompareInt _setoutsidedoorspeed 5
        (:==
          (Variables|Default|SetFinalOutsideDoorSpeed Speed_05))))))

(event Custom|ArrowDisplayDoorFrame
  (params (DoorFrameZAxis :type Float%20%28double-precision%29) (EleavatorZAxis :type Float%20%28double-precision%29))
  (bind _displayarrow (Variables|Default|GetDisplayArrow))
  ;[1 1 1] Arrow display door frame
  ;;[0.1744 1 0] Receive elevator and door frame Z axis from "BP_Elevator" and compare to see if its going up or down to show the right direction.
  (if (Math|Float|NearlyEqual(Float) DoorFrameZAxis EleavatorZAxis 1e+01)
    (Rendering|Material|SetMaterial _displayarrow 0 "/Game/ElevatorSystem/Material/Instances/ArrowDisplay/1K/MI_ArrowDisplay_1K_01.MI_ArrowDisplay_1K_01")
    (else
      (Math|Float|CompareFloat DoorFrameZAxis EleavatorZAxis
        (:>
          (Rendering|Material|SetMaterial _displayarrow 0 "/Game/ElevatorSystem/Material/Instances/ArrowDisplay/1K/MI_ArrowDisplay_1K_03.MI_ArrowDisplay_1K_03"))
        (:<
          (Rendering|Material|SetMaterial _displayarrow 0 "/Game/ElevatorSystem/Material/Instances/ArrowDisplay/1K/MI_ArrowDisplay_1K_02.MI_ArrowDisplay_1K_02"))))))

(event Custom|Call%20Button%20Light%20Up
  (bind _callbuttonup (Variables|Default|GetCallButtonUp))
  ;[1 1 1] Call button light
  ;;[0.1744 1 0] Change the material to turn the button light on or off.
  (if (Variables|Default|GetCallButtonUpLightOn)
    (Rendering|Material|SetMaterial _callbuttonup 0 "/Game/ElevatorSystem/Material/Instances/ButtonLight/MI_ButtonLight_03.MI_ButtonLight_03")
    (Rendering|Material|SetMaterial (Variables|Default|GetCallButtonDown) 0 "/Game/ElevatorSystem/Material/Instances/ButtonLight/MI_ButtonLight_02.MI_ButtonLight_02")
    (else
      (Rendering|Material|SetMaterial _callbuttonup 0 "/Game/ElevatorSystem/Material/Instances/ButtonLight/MI_ButtonLight_02.MI_ButtonLight_02"))))

(event Custom|PushCallButtonDown
  (bind _callbuttondown (Variables|Default|GetCallButtonDown))
  (bind _relativelocation (Variables|/Script/Engine.SceneComponent|GetRelativeLocation _callbuttondown))
  (bind (_x _y _z) (Math|Vector|BreakVector _relativelocation))
  ;[1 1 1] Push call button down
  ;;[0.1744 1 0] Store the initial button location on "ButtonPosition", move the button and move back to the initial location.
  (Audio|Components|Audio|Play (Variables|Default|GetButtonNoise) 0.0)
  (if (Variables|Default|GetCanPushCallButton)
    (Audio|Components|Audio|Play (Variables|Default|GetButtonBip) 0.0)
    (Variables|Default|SetCanPushCallButton false)
    (bind _output_get (Variables|Default|SetButtonPosition _relativelocation))
    (bind _alpha (Timeline|Timeline_1 PlayFromStart)
      (:Update
        (Transformation|SetRelativeLocation _callbuttondown (Math|Vector|MakeVector _x (Math|Float|Lerp _y (- _y 0.07) _alpha) _z) false false))
      (:Finished
        (bind _alpha_2 (Timeline|Timeline_2 PlayFromStart)
          (:Update
            (Transformation|SetRelativeLocation _callbuttondown (Math|Vector|MakeVector (.X (Math|Vector|BreakVector _output_get)) (Math|Float|Lerp (Math|Float|Lerp _y (- _y 0.07) _alpha) (.Y (Math|Vector|BreakVector _output_get)) _alpha_2) (.Z (Math|Vector|BreakVector _output_get))) false false))
          (:Finished
            (Variables|Default|SetCanPushCallButton true)))))))

(event EventBeginPlay
  (bind _floorplatenumber (Variables|Default|GetFloorPlateNumber))
  (bind _doorframewall_01 (Variables|Default|GetDoorFrameWall_01))
  (bind _doorframewall_02 (Variables|Default|GetDoorFrameWall_02))
  (bind _doorframewall_03 (Variables|Default|GetDoorFrameWall_03))
  ;[1 1 1] Event begin play.
  ;;[0.1744 1 0] Set wall shaft collision
  (Utilities|FlowControl|Sequence
    (:then_0
      (if (Variables|Parameters|GetAddShaftWall_01)
        (Collision|SetCollisionEnabled _doorframewall_01 "QueryAndPhysics")
        (else
          (Collision|SetCollisionEnabled _doorframewall_01 "NoCollision"))))
    (:then_1
      (if (Variables|Parameters|GetAddShaftWall_02)
        (Collision|SetCollisionEnabled _doorframewall_02 "QueryAndPhysics")
        (else
          (Collision|SetCollisionEnabled _doorframewall_02 "NoCollision"))))
    (:then_2
      (if (Variables|Parameters|GetAddShaftWall_03)
        (Collision|SetCollisionEnabled _doorframewall_03 "QueryAndPhysics")
        (else
          (Collision|SetCollisionEnabled _doorframewall_03 "NoCollision"))))
    (:then_3
      (if (Variables|Parameters|GetFloorPlateVisibility)
        (Collision|SetCollisionEnabled _floorplatenumber "QueryAndPhysics")
        (else
          (Collision|SetCollisionEnabled _floorplatenumber "NoCollision"))))))

(fn ConstructionScript
  (bind _floorplatenumber (Variables|Default|GetFloorPlateNumber))
  (bind _floorplatevisibility (Variables|Parameters|GetFloorPlateVisibility))
  (bind _addshaftwall_03 (Variables|Parameters|GetAddShaftWall_03))
  (bind _doorframewall_01 (Variables|Default|GetDoorFrameWall_01))
  (bind _addshaftwall_01 (Variables|Parameters|GetAddShaftWall_01))
  (bind _doorframewall_02 (Variables|Default|GetDoorFrameWall_02))
  (bind _doorframewall_03 (Variables|Default|GetDoorFrameWall_03))
  (bind _addshaftwall_02 (Variables|Parameters|GetAddShaftWall_02))
  ;[0.1744 1 0] Set wall shaft and floor plate visibility
  (Utilities|FlowControl|Sequence
    (:then_0
      (if _addshaftwall_01
        (Rendering|SetVisibility _doorframewall_01 _addshaftwall_01 false)
        (else
          (Rendering|SetVisibility _doorframewall_01 _addshaftwall_01 false))))
    (:then_1
      (if _addshaftwall_02
        (Rendering|SetVisibility _doorframewall_02 _addshaftwall_02 false)
        (else
          (Rendering|SetVisibility _doorframewall_02 _addshaftwall_02 false))))
    (:then_2
      (if _addshaftwall_03
        (Rendering|SetVisibility _doorframewall_03 _addshaftwall_03 false)
        (else
          (Rendering|SetVisibility _doorframewall_03 _addshaftwall_03 false))))
    (:then_3
      (if _floorplatevisibility
        (Rendering|SetVisibility _floorplatenumber _floorplatevisibility false)
        (else
          (Rendering|SetVisibility _floorplatenumber _floorplatevisibility false))))))